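; BP_ClockManager is a manager Blueprint for BP_Clock actors, but its spawn and registration logic is disconnected and BeginPlay does nothing.
; The unwired chain spawns three clocks at random heights, then binds every BP_Clock's OnClockAlert dispatcher to a local event.
; That event prints the received Cuckoo value.
; A stray cast of the game mode to GM_New is also unconnected.
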(event Custom|OnClockAlert_Event
  (params (Cuckoo :type Boolean))
  (Development|PrintString (Utilities|String|Append "clock =" (Utilities|String|ToString(Boolean) Cuckoo))))

(event EventBeginPlay)

(fn ConstructionScript)