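; Player controller that turns Enhanced Input actions into movement, look, jump and shooting for player 0.
; BeginPlay adds the IMC_MyContext mapping, then the action events drive pawn movement, controller yaw and pitch, and character jump.
; Shooting spawns a small BP_Bullet at BP_CustomPlayer's BarrelEdge and launches it with a physics impulse along the barrel's forward vector.
; Array, set and map nodes are unconnected and never run.
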(event Input|EnhancedActionEvents|EnhancedInputActionIA_Shoot
  (params (ActionValue :type Boolean) (ElapsedSeconds :type Float%20%28double-precision%29) (TriggeredSeconds :type Float%20%28double-precision%29) (InputAction :type Input%20Action%20Object%20Reference :default "/Game/Input/IA_Shoot.IA_Shoot"))
  (bind _asbp_custom_player (Utilities|Casting|CastToBP_CustomPlayer (Game|Player|GetPlayerPawn 0)))
  (bind _returnvalue (Game|SpawnActorfromClass "/Game/Blueprints/BP_Bullet.BP_Bullet_C" (Math|Transform|MakeTransform (Transformation|GetWorldLocation (Variables|/Game/Blueprints/BP_CustomPlayer.BP_CustomPlayer_C|GetBarrelEdge _asbp_custom_player)) "0, 0, 0" "0.100000,0.100000,0.100000") "AlwaysSpawn" "MultiplyWithRoot" 0 1e+02 0))
  (Physics|SetSimulatePhysics (Variables|/Script/Engine.StaticMeshActor|GetStaticMeshComponent _returnvalue) true)
  (Physics|AddImpulse (Variables|/Script/Engine.StaticMeshActor|GetStaticMeshComponent _returnvalue) (* (Math|Vector|GetForwardVector (Variables|/Game/Blueprints/BP_CustomPlayer.BP_CustomPlayer_C|GetBarrelEdge _asbp_custom_player)) 1e+06) "None" false))

(event Input|EnhancedActionEvents|EnhancedInputActionIA_Look
  (params (ActionValue :type Vector%202D%20Structure) (ElapsedSeconds :type Float%20%28double-precision%29) (TriggeredSeconds :type Float%20%28double-precision%29) (InputAction :type Input%20Action%20Object%20Reference :default "/Game/Input/IA_Look.IA_Look"))
  (Class|PlayerController|AddYawInput (.y ActionValue))
  (Class|PlayerController|AddPitchInput (.x ActionValue)))

(event Input|EnhancedActionEvents|EnhancedInputActionIA_Move
  (params (ActionValue :type Vector%202D%20Structure) (ElapsedSeconds :type Float%20%28double-precision%29) (TriggeredSeconds :type Float%20%28double-precision%29) (InputAction :type Input%20Action%20Object%20Reference :default "/Game/Input/IA_Move.IA_Move"))
  (bind _returnvalue (Game|Player|GetPlayerPawn 0))
  (Pawn|Input|AddMovementInput _returnvalue (Transformation|GetActorForwardVector _returnvalue) (.x ActionValue) false)
  (Pawn|Input|AddMovementInput _returnvalue (Transformation|GetActorRightVector _returnvalue) (.y ActionValue) false))

(event Input|EnhancedActionEvents|EnhancedInputActionIA_Jump
  (params (ActionValue :type Boolean) (ElapsedSeconds :type Float%20%28double-precision%29) (TriggeredSeconds :type Float%20%28double-precision%29) (InputAction :type Input%20Action%20Object%20Reference :default "/Game/Input/IA_Jump.IA_Jump"))
  (Character|Jump (Game|GetPlayerCharacter 0)))

(event EventBeginPlay
  (Input|AddMappingContext (PlayerController|LocalPlayerSubsystems|GetEnhancedInputLocalPlayerSubsystem) "/Game/Input/IMC_MyContext.IMC_MyContext" 0 "(bIgnoreAllPressedKeysUntilRelease=True,bForceImmediately=False,bNotifyUserSettings=False)"))

(event EventTick
  (params (DeltaSeconds :type Float%20%28single-precision%29)))

(fn ConstructionScript)