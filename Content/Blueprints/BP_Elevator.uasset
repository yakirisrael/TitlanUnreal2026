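; BP_Elevator is a moving elevator actor that rises above its starting position while widening horizontally.
; On BeginPlay it stores its location and plays the UpAndDown timeline from the start.
; Each timeline update offsets Z by Alpha times Speed and MaxHeight, so Speed scales travel distance rather than timing.
; The same Alpha drives X and Y scale, with no sweep on movement.
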(event EventBeginPlay
  (Variables|Default|SetStartPosition (Transformation|GetActorLocation))
  (bind _alpha (Timeline|UpAndDown PlayFromStart)
    (:Update
      (Transformation|SetActorLocation (Math|Vector|MakeVector (.x (Variables|Default|GetStartPosition)) (.y (Variables|Default|GetStartPosition)) (+ (.z (Variables|Default|GetStartPosition)) (* (* (Variables|Default|GetSpeed) 1.0 _alpha) (Variables|Default|GetMaxHeight)))) false false)
      (Transformation|SetActorScale3D (Math|Vector|MakeVector (+ (* _alpha 1.5) 1.0) (+ (* _alpha 1.5) 1.0) 1.0)))))

(event Collision|EventActorBeginOverlap
  (params (OtherActor :type Actor%20Object%20Reference)))

(event EventTick
  (params (DeltaSeconds :type Float%20%28single-precision%29)))

(fn ConstructionScript)