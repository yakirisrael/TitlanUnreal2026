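; Enemy Blueprint that tests whether the player is inside its forward view cone and prints the result every Tick as debug output.
; IsSeePlayerInRange compares the dot product of forward and direction-to-player against Range, an angular threshold with no distance or occlusion check.
; The same function also turns Arrow1 toward the player, ignoring pitch.
; Unconnected leftover nodes hold experiments for AI MoveTo chasing, smoothed look-at rotation and a forward line trace.
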(event EventBeginPlay)

(event Collision|EventActorBeginOverlap
  (params (OtherActor :type Actor%20Object%20Reference)))

(event EventTick
  (params (DeltaSeconds :type Float%20%28single-precision%29))
  (Development|PrintString (Utilities|String|ToString(Boolean) (CallFunction|IsSeePlayerinRange 0.7))))

(fn ConstructionScript)

(fn IsSeePlayerinRange
  (params (range' :type Float%20%28double-precision%29))
  (bind _returnvalue (Game|Player|GetPlayerPawn 0))
  (bind _returnvalue_2 (Transformation|GetActorLocation))
  (bind _returnvalue_3 (Transformation|GetActorLocation _returnvalue))
  (bind _returnvalue_4 (- _returnvalue_3 _returnvalue_2))
  (bind _returnvalue_5 (Math|Conversions|RotationFromXVector _returnvalue_4))
  (Transformation|SetWorldRotation (Variables|Default|GetArrow1) (Math|Rotator|MakeRotator (.roll _returnvalue_5) 0.0 (.yaw _returnvalue_5)) false false)
  (return (> (Math|Vector|DotProduct (Transformation|GetActorForwardVector) (Math|Vector|Normalize _returnvalue_4)) range')))